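; Player controller that runs a voice chat pipeline for a talking head and drives the main UI.
; Prompts go to a local LM Studio LLM over HTTP, and the streamed reply is queued and split at sentence marks.
; Chunks feed ElevenLabs websocket TTS, whose PCM and character data become lipsync phrases for SpeakingHead.
; An Idle/Text/Audio/Speak state machine paces requests and re-enables the microphone; the OpenAI variant is an unused demo.
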(event `SetGenerationState`
  (params (NewState :type "/Game/Blueprins/E_State Enum" :default "NewEnumerator0"))
  (bind _mainui (`self.MainUI`))
  ;[1 1 1] Set generation state and update UI
  (bind _output_get (set `self.State` NewState))
  (`/Game/UI/W_Main.UpdateStateWidget` (`self.MainUI`) _output_get)
  (switch `/Game/Blueprins/E_State` _output_get
    (:`NewEnumerator0`
      (`/Game/UI/W_Main.ResetGenerationUI` _mainui)
      (if (`CheckBox.IsChecked` (`/Game/UI/W_Main.CB_Microphone` _mainui))
        (`KismetSystemLibrary.Delay` 0.5)
        (bind _asbp_spectator_player (cast `/Game/Blueprins/BP_SpectatorPlayer` (`self.K2_GetPawn`)))
        (`/Game/Blueprins/BP_SpectatorPlayer.SetMicrophonEnabled` _asbp_spectator_player true)))))

(event `self.ReceiveBeginPlay`
  (bind _returnvalue (subsystem `HTTPSubsystem`))
  (`|ExecutionSequence`
    (:`then_0`
      ;[1 1 1] Create UI
      (bind _returnvalue_2 (`|CreateWidget` "/Game/UI/W_Main.W_Main_C" self))
      (bind _output_get (set `self.MainUI` _returnvalue_2))
      (`UserWidget.AddToViewport` _output_get 0)
      (`WidgetBlueprintLibrary.SetInputMode_UIOnlyEx` self (`self.MainUI`))
      (set `self.bShowMouseCursor` true))
    (:`then_1`
      ;[1 1 1] Bind to HTTP Events
      (add `HTTPSubsystem.OnTextResponse` _returnvalue (delegate `OnHttp_ResponseText`))
      (add `HTTPSubsystem.OnTextStreamResponse` _returnvalue (delegate `OnHttp_TextStream`))
      (set `HTTPSubsystem.bResponseInGameThread` false _returnvalue))))

(event `OnHttp_TextStream`
  (params (RequestName :type "Name (by ref)") (Text :type String))
  ; Received Text Chunk: feed it to 11Labs and finalize on sentence end
  (`self.ProcessGeneratedTextDelta` (`JsonItemFunctionsLibrary.JsonGetFieldValue_String` (`JsonItemFunctionsLibrary.JsonItemFromString` Text) "choices[0].delta.content")))

(event `OnHttp_ResponseText`
  (params (RequestName :type "Name (by ref)") (Code :type Integer) (Headers :type "Array of String (by ref)") (Data :type String))
  (bind (_text _remained) (`self.GetAvailableData` true))
  (bind _bwaitingforaudioresult (`self.bWaitingForAudioResult`))
  ;[1 1 1] Process data returned via HTTP (called when stream finished)
  (switch `/Game/Blueprins/E_State` (`self.State`)
    (:`NewEnumerator1`
      (if (`KismetStringLibrary.IsEmpty` _text)
        (if _bwaitingforaudioresult
          (`self.SetGenerationState` "NewEnumerator2")
          (else
            (`self.SetGenerationState` "NewEnumerator3")))
        (else
          (`self.SetGenerationState` "NewEnumerator2")
          (if (not _bwaitingforaudioresult)
            (`self.Request_TTS` _text true)
            (`self.ClearSentenceQueue` _remained)))))))

(event `Request_TTS`
  (params (Text :type String) (bFinal :type Boolean))
  ; Send Streamed Request to ElevenLabs via Websocket
  (bind _output_get (set `self.AccumulatedTTSOutput` (`KismetStringLibrary.Concat_StrStr` (`self.AccumulatedTTSOutput`) Text)))
  (`self.UI_TextSent` Text)
  (if (not (`KismetStringLibrary.IsEmpty` (`KismetStringLibrary.Trim` _output_get)))
    (`TextToSpeechStreamPlayer.GenerateTextChunk` (`self.TextToSpeechStreamPlayer`) Text bFinal)
    (set `self.bWaitingForAudioResult` (or bFinal (`self.bWaitingForAudioResult`)))))

(event `ProcessGeneratedTextDelta`
  (params (TextDelta :type String))
  (bind (_bsplitted _a _b) (`self.SplitTokenByMark` TextDelta))
  (bind (_text _remained) (`self.GetAvailableData` (`self.bFinalChunkInSentence`)))
  ; Process Streamed Text Data
  (`self.UI_TextGenerated` TextDelta)
  (`self.AppendToSentence` _a)
  (bind _output_get (set `self.bFinalChunkInSentence` _bsplitted))
  (if _output_get
    (`|ExecutionSequence`
      (:`then_0`
        (if (not (`self.bWaitingForAudioResult`)) :!label _label
          (set `self.bFinalChunkInSentence` (or (`self.bFinalChunkInSentence`) (> (`self.GetSentenceEndIndex` (`self.SentenceQueue`)) 0)))
          (if (not (`KismetStringLibrary.IsEmpty` _text))
            (`self.Request_TTS` _text (`self.bFinalChunkInSentence`))
            (`self.ClearSentenceQueue` _remained))))
      (:`then_1`
        (`self.AppendToSentence` _b)))
    (else
      (goto _label))))

(event `SubmitNewPrompt`
  (params (Text :type String))
  ;[1 0.3958 0.3958] Generate Text (local LLM via LM Studio)
  (switch `/Game/Blueprins/E_State` (`self.State`)
    (:`NewEnumerator0`
      (`self.SetGenerationState` "NewEnumerator1")
      (`self.UI_Prompt` Text)
      (bind _output_get (set `self.CurrentRequest` (`JsonItemFunctionsLibrary.JsonItemFromString` (`self.Template_LMStudio`))))
      (`JsonItemFunctionsLibrary.JsonSetFieldValue_String` _output_get "messages[role=user].content" Text)
      (`HTTPSubsystem.SendHttpRequest` (subsystem `HTTPSubsystem`) "OpenAI" (`self.Endpoint_LMStudio`) "Post" (`|MakeArray` (`JsonItemFunctionsLibrary.GetDefaultContentAppJson`)) (`JsonItemFunctionsLibrary.JsonItemToString` (`self.CurrentRequest`)) "StreamText")
      (`/Game/UI/W_Main.ResetGenerationUI` (`self.MainUI`)))))

(event `SubmitNewPrompt_2`
  (params (Text :type String))
  ;[1 0.3958 0.3958] DEMO (not in use): Request to api.openai.com.
  (switch `/Game/Blueprins/E_State` (`self.State`)
    (:`NewEnumerator0`
      (`self.SetGenerationState` "NewEnumerator1")
      (bind _output_get (set `self.CurrentRequest` (`JsonItemFunctionsLibrary.JsonItemFromString` (`self.Template_OpenAI`))))
      (`JsonItemFunctionsLibrary.JsonSetFieldValue_String` _output_get "messages[role=user].content" Text)
      (`JsonItemFunctionsLibrary.JsonSetFieldValue_String` (`self.CurrentRequest`) "messages[role=developer].content" "[put your dev instruction here]")
      (`JsonItemFunctionsLibrary.JsonSetFieldValue_String` (`self.CurrentRequest`) "model" "gpt-4o-mini")
      (`HTTPSubsystem.SendHttpRequest` (subsystem `HTTPSubsystem`) "OpenAI" (`self.Endpoint_OpenAI`) "Post" (`|MakeArray` (`JsonItemFunctionsLibrary.GetDefaultContentAppJson`) (make `YnnkUrlParameter` "Authorization:" (`KismetStringLibrary.Concat_StrStr` "Bearer " "[insert your API key here]"))) (`JsonItemFunctionsLibrary.JsonItemToString` (`self.CurrentRequest`)) "StreamText"))))

(event `SubmitTTSRequest`
  (params (Text :type String))
  ;[0.4461 1 0.4314] Generate Voice
  (switch `/Game/Blueprins/E_State` (`self.State`)
    (:`NewEnumerator1`
      (`self.SetGenerationState` "NewEnumerator2")
      (set `self.CurrentRequest` (`JsonItemFunctionsLibrary.JsonItemFromString` (`self.Template_TTS`)))
      (`JsonItemFunctionsLibrary.JsonSetFieldValue_String` (`self.CurrentRequest`) "data[2]" (`KismetStringLibrary.Concat_StrStr` (`KismetSystemLibrary.GetProjectDirectory`) "voice_ref.wav"))
      (`JsonItemFunctionsLibrary.JsonSetFieldValue_String` (`self.CurrentRequest`) "data[1]" Text)
      (`HTTPSubsystem.SendHttpRequest` (subsystem `HTTPSubsystem`) "TTS" "http://localhost:5003/run/run_tts" "Post" (`|MakeArray` (`JsonItemFunctionsLibrary.GetDefaultContentAppJson`)) (`JsonItemFunctionsLibrary.JsonItemToString` (`self.CurrentRequest`)) "Default"))))

(event `self.TextToSpeechStreamPlayer.OnGenerationComplete`
  (params (FullVoiceSound :type "SoundWave Object Reference") (PCMData :type "Array of Byte (by ref)") (Characters :type "Array of GeneratedCharacter Structure (by ref)"))
  ;[0.08239 0.2273 1] Receive and Play Generated Voice
  (if (not (`KismetArrayLibrary.Array_IsEmpty` PCMData))
    (bind _returnvalue (`YnnkLipSyncFunctionLibrary.CreateLipsyncForRecognizedAudio` self (`YnnkLipSyncFunctionLibrary.CreateRuntimeSoundWave` self 44100 PCMData) "VRD_Characters" (`ElevenVoiceFunctionLibrary.GetCharactersDataAsJson` Characters) true))
    (`self.UI_AudioGenerated` _returnvalue)
    (message `/Game/Blueprins/SpeakActorInterface.NextPhrase` (`self.SpeakingHead`) _returnvalue)))

(event `self.TextToSpeechStreamPlayer.OnWinsocketReady`
  (bind (_text _remained) (`self.GetAvailableData` true))
  ;[0.08239 0.2273 1] Generate Next Sentence or Allow to generate from SubmitNewPrompt
  (if (`self.bWaitingForAudioResult`) :!label _label_2
    (set `self.bWaitingForAudioResult` false)
    (if (`|EnumEquality` (`self.State`) "NewEnumerator2")
      (if (`KismetStringLibrary.IsEmpty` (`self.SentenceQueue`))
        (`self.SetGenerationState` "NewEnumerator3")
        (else
          (`self.Request_TTS` _text true)
          (`self.ClearSentenceQueue` _remained))))))

(event `Debug_DummyTTS`
  ;[0.08239 0.2273 1] Generate Next Sentence or Allow to generate from SubmitNewPrompt
  (goto _label_2))

(fn `GetAvailableData`
  (params (bFInalizingSentence :type Boolean))
  (returns (Text :type String) (Remained :type String))
  (locals (OutData :type String))
  (bind _returnvalue (`KismetStringLibrary.FindSubstring` (`local.OutData`) " " false true))
  (bind _delimiterindex (`self.GetSentenceEndIndex` (`self.SentenceQueue`)))
  (bind (_left _right) (`self.SplitTextByIndex` (`local.OutData`) _returnvalue))
  (bind (_left_2 _right_2) (`self.SplitTextByIndex` (`self.SentenceQueue`) _delimiterindex))
  ; True - split to return first complete sentence
  ; False - split to last complete word
  (if bFInalizingSentence
    (if (> _delimiterindex 0)
      (return _left_2 _right_2)
      (else
        (return (`self.SentenceQueue`) "")))
    (else
      (set `local.OutData` (`self.SentenceQueue`))
      (if (> _returnvalue 0)
        (return _left _right)
        (else
          (return "" (`local.OutData`)))))))

(fn `SplitTokenByMark`
  (params (Source :type String))
  (returns (bSplitted :type Boolean) (A :type String) (B :type String))
  (locals (Separators :type "Array of String"))
  (for _array_element (`local.Separators`)
    (bind (_lefts _rights _returnvalue) (`KismetStringLibrary.Split` (`local.Source`) _array_element))
    (if _returnvalue
      (return true (`KismetStringLibrary.Concat_StrStr` _lefts _array_element) _rights)))
  (return false (`local.Source`) ""))

(fn `UserConstructionScript`)