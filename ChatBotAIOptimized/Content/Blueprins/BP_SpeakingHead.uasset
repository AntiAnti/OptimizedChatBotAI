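; BP_SpeakingHead is a talking head actor that voices lipsync phrases through a YnnkLipsyncController and registers itself with BP_PlayerController on BeginPlay.
; NextPhrase speaks incoming lipsync data immediately, or queues it if speech is already playing.
; When each phrase completes it plays the next queued one in order, and once the queue is empty it sets the player controller's generation state to signal completion.
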(event `self.ReceiveBeginPlay`
  (bind _asbp_player_controller (cast `/Game/Blueprins/BP_PlayerController` (`GameplayStatics.GetPlayerController` 0)))
  (set `/Game/Blueprins/BP_PlayerController.SpeakingHead` self _asbp_player_controller))

(event `/Game/Blueprins/SpeakActorInterface.NextPhrase`
  (params (LipsyncData :type "YnnkVoiceLipsyncData Object Reference"))
  ; Speak Next
  (if (`YnnkLipsyncController.IsSpeaking` (`self.YnnkLipsyncController`))
    (`KismetArrayLibrary.Array_Add` (`self.Queue`) LipsyncData)
    (else
      (`YnnkLipsyncController.Speak` (`self.YnnkLipsyncController`) LipsyncData))))

(event `self.YnnkLipsyncController.OnSpeakingComplete`
  (params (PhraseAsset :type "YnnkVoiceLipsyncData Object Reference"))
  ; Notify player controller that the phrase is finished
  (if (`KismetArrayLibrary.Array_IsEmpty` (`self.Queue`))
    (bind _asbp_player_controller (cast `/Game/Blueprins/BP_PlayerController` (`GameplayStatics.GetPlayerController` 0)))
    (`/Game/Blueprins/BP_PlayerController.SetGenerationState` _asbp_player_controller "NewEnumerator0")
    (else
      (`YnnkLipsyncController.Speak` (`self.YnnkLipsyncController`) (`|GetArrayItem` (`self.Queue`)))
      (`KismetArrayLibrary.Array_Remove` (`self.Queue`)))))

(fn `UserConstructionScript`)