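; BP_SpectatorPlayer is the player's spectator class that turns microphone speech into prompts.
; SetMicrophonEnabled starts or stops streaming voice capture while BP_PlayerController is Idle.
; Recognized text is cached and shown in yellow in the controller's main UI.
; A retriggerable delay detects a one-second pause in recognition, then, if still Idle, stops capture and submits the text to the controller as a new prompt.
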(event `SetMicrophonEnabled`
  (params (bNewEnabled :type Boolean))
  (bind _streamvoicerecognize (`self.StreamVoiceRecognize`))
  (bind _asbp_player_controller (cast `/Game/Blueprins/BP_PlayerController` (`GameplayStatics.GetPlayerController` 0)))
  (switch `/Game/Blueprins/E_State` (`/Game/Blueprins/BP_PlayerController.State` _asbp_player_controller)
    (:`NewEnumerator0`
      (if bNewEnabled
        (`StreamVoiceRecognizeComponent.StartCapture` _streamvoicerecognize)
        (else
          (`StreamVoiceRecognizeComponent.StopCapture` _streamvoicerecognize false))))))

(event `self.StreamVoiceRecognize.OnVoiceDataRecognized`
  (params (bIsFinalized :type Boolean) (Text :type String))
  (bind _output_get (set `self.CachedText` Text))
  (bind _asbp_player_controller (cast `/Game/Blueprins/BP_PlayerController` (`GameplayStatics.GetPlayerController` 0)))
  (bind _tb_prdata (`/Game/UI/W_Main.TB_PrData` (`/Game/Blueprins/BP_PlayerController.MainUI` _asbp_player_controller)))
  (`TextBlock.SetText` _tb_prdata (`KismetTextLibrary.Conv_StringToText` _output_get))
  (`TextBlock.SetColorAndOpacity` _tb_prdata (make `SlateColor` (struct :`R` 1.0 :`G` 0.892731 :`B` 0.289067 :`A` 1.0)))
  ; Wait for 1 sec pause
  (`KismetSystemLibrary.RetriggerableDelay` 1.0)
  (bind _asbp_player_controller_2 (cast `/Game/Blueprins/BP_PlayerController` (`GameplayStatics.GetPlayerController` 0)))
  (switch `/Game/Blueprins/E_State` (`/Game/Blueprins/BP_PlayerController.State` _asbp_player_controller_2)
    (:`NewEnumerator0`
      (`StreamVoiceRecognizeComponent.StopCapture` (`self.StreamVoiceRecognize`) false)
      (`/Game/Blueprins/BP_PlayerController.SubmitNewPrompt` _asbp_player_controller_2 (`self.CachedText`))
      (set `self.CachedText` ""))))

(fn `UserConstructionScript`)